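; Networked gun actor, attached to a parent player character, that handles firing, magazine ammo, reloading and accuracy-based shot spread.
; The server runs the fire-rate cooldown and ammo count, with a RepNotify updating the owning client's HUD.
; Fire traces a predicted projectile path with debug drawing and plays sound, plus an arms montage on hit.
; Only the server applies damage, through the hit actor's HealthComponent.
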(event `self.ReceiveBeginPlay`
  (set `self.RoundsRemainingInMagazine` (`self.MagazineSize`)))

(event `self.ReceiveTick`
  (params (DeltaSeconds :type "Float (single-precision)"))
  (if (not (`self.RoundsInitialised`))
    (`/Engine/EditorBlueprintResources/StandardMacros.IsValid` (`self.GetParentActor`)
      (:`Is Valid`
        (`self.UpdateRounds`)
        (set `self.RoundsInitialised` true))))
  (`/Engine/EditorBlueprintResources/ActorMacros.Switch Has Authority`
    (:`Authority`
      (if (not (`self.bCanFire`))
        (bind _output_get (set `self.TimeTillNextShot` (- (`self.TimeTillNextShot`) DeltaSeconds)))
        (if (<= _output_get 0.0)
          (set `self.bCanFire` (> (`self.RoundsRemainingInMagazine`) 0)))))))

(fn `CalculateShotDirection`
  (params (OriginalDirection :type "Vector Structure"))
  (returns (LaunchDirection :type "Vector Structure"))
  (return (* (`KismetMathLibrary.Normal` (+ (`KismetMathLibrary.RandomUnitVector`) (* OriginalDirection (`self.WeaponAccuracy`)))) (`self.MuzzleVelocity`))))

(fn `Fire`
  (params (LaunchDirection :type "Vector Structure"))
  (bind _returnvalue (`SceneComponent.K2_GetComponentLocation` (`self.MuzzlePosition`)))
  (if (`self.bCanFire`)
    (`/Engine/EditorBlueprintResources/ActorMacros.Switch Has Authority`
      (:`Authority`
        (set `self.bCanFire` false)
        (set `self.TimeTillNextShot` (`self.FireRate`))
        (set `self.RoundsRemainingInMagazine` (- (`self.RoundsRemainingInMagazine`) 1)))
      (:`Remote`
        _))
    (bind (_outhit _outpathpositions _outlasttracedestination _returnvalue_2) (`GameplayStatics.Blueprint_PredictProjectilePath_ByTraceChannel` :`StartPos` _returnvalue :`LaunchVelocity` (* LaunchDirection (`self.MuzzleVelocity`)) :`ProjectileRadius` 1.0 :`DrawDebugType` "ForDuration" :`DrawDebugTime` 4.0))
    (`GameplayStatics.PlaySoundAtLocation` "/Game/Assets/Audio/FirstPersonTemplateWeaponFire02.FirstPersonTemplateWeaponFire02" _returnvalue (struct) 1.0 1.0 0.0 null null null)
    (if _returnvalue_2
      (bind _asplayer_character_blueprint (cast `/Game/Blueprints/PlayerCharacterBlueprint` (`self.GetParentActor`))
        (:`then`
          (`AnimInstance.Montage_Play` (`SkeletalMeshComponent.GetAnimInstance` (`/Game/Blueprints/PlayerCharacterBlueprint.Arms` _asplayer_character_blueprint)) "/Game/Assets/Arms/Animations/FirstPersonFire_Montage.FirstPersonFire_Montage" 1.0 "MontageLength" 0.0 true))
        (:`CastFailed`
          _))
      (bind (_bblockinghit _binitialoverlap _time _distance _location _impactpoint _normal _impactnormal _physmat _hitactor) (`GameplayStatics.BreakHitResult` _outhit))
      (if (and (`KismetSystemLibrary.IsServer`) (`KismetSystemLibrary.IsValid` _hitactor) _returnvalue_2)
        (bind _returnvalue_3 (`self.GetComponentByClass` _hitactor "/Script/AdvGamesProgramming.HealthComponent"))
        (if (`KismetSystemLibrary.IsValid` _returnvalue_3)
          (`HealthComponent.OnTakeDamage` _returnvalue_3 (`self.BulletDamage`))
          (`KismetSystemLibrary.PrintString` (`KismetStringLibrary.Conv_DoubleToString` (`HealthComponent.CurrentHealth` _returnvalue_3)))
          (else
            (`KismetSystemLibrary.PrintString` "Did not hit actor with health component" true false)))))))

(fn `OnRep_RoundsRemainingInMagazine`
  (`self.UpdateRounds`))

(fn `Reload`
  (set `self.RoundsRemainingInMagazine` (`self.MagazineSize`)))

(fn `UpdateRounds`
  (bind _returnvalue (`self.GetParentActor`))
  (`/Engine/EditorBlueprintResources/StandardMacros.IsValid` _returnvalue
    (:`Is Valid`
      (if (`|EnumEquality` (`self.GetLocalRole` _returnvalue) "ROLE_AutonomousProxy")
        (bind _asplayer_hud (cast `PlayerHUD` (`PlayerController.GetHUD` (`GameplayStatics.GetPlayerController` 0))))
        (`PlayerHUD.SetPlayerRounds` _asplayer_hud (`self.RoundsRemainingInMagazine`) (`self.MagazineSize`))))))

(fn `UserConstructionScript`)