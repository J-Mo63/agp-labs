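; GunBlueprint is a player-held gun whose Fire function launches a predicted shot from its muzzle.
; Fire traces a projectile path from MuzzlePosition along the given direction scaled by MuzzleVelocity, drawing it as debug for a few seconds; the result is unused.
; It then plays a fire sound and, through its parent PlayerCharacterBlueprint, plays the fire montage on the arms.
; No projectile is spawned and no damage is applied.
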(fn `Fire`
  (params (LaunchDirection :type "Vector Structure"))
  (bind _returnvalue (`SceneComponent.K2_GetComponentLocation` (`self.MuzzlePosition`)))
  (`GameplayStatics.Blueprint_PredictProjectilePath_ByTraceChannel` :`StartPos` _returnvalue :`LaunchVelocity` (* LaunchDirection (`self.MuzzleVelocity`)) :`ProjectileRadius` 1.0 :`DrawDebugType` "ForDuration" :`DrawDebugTime` 4.0)
  (`GameplayStatics.PlaySoundAtLocation` "/Game/Assets/Audio/FirstPersonTemplateWeaponFire02.FirstPersonTemplateWeaponFire02" _returnvalue (struct) 1.0 1.0 0.0 null null null)
  (bind _asplayer_character_blueprint (cast `/Game/Blueprints/PlayerCharacterBlueprint` (`self.GetParentActor`)))
  (`AnimInstance.Montage_Play` (`SkeletalMeshComponent.GetAnimInstance` (`/Game/Blueprints/PlayerCharacterBlueprint.Arms` _asplayer_character_blueprint)) "/Game/Assets/Arms/Animations/FirstPersonFire_Montage.FirstPersonFire_Montage" 1.0 "MontageLength" 0.0 true))

(fn `UserConstructionScript`)