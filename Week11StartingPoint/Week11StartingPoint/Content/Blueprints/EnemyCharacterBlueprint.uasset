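; Enemy character Blueprint that shoots and reloads a GunBlueprint held in its Gun child actor component.
; Tick polls the gun's magazine to keep the OutOfAmmo flag current.
; Fire adds random spread scaled by TargetAccuracyOffset to the given direction, then rotates the actor toward the unperturbed direction.
; Reload blocks firing, plays a montage, and uses its returned length as the delay before refilling the gun.
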(event `self.ReceiveTick`
  (params (DeltaSeconds :type "Float (single-precision)"))
  (bind _asgun_blueprint (cast `/Game/Blueprints/GunBlueprint` (`ChildActorComponent.ChildActor` (`self.Gun`))))
  (if (<= (`/Game/Blueprints/GunBlueprint.RoundsRemainingInMagazine` _asgun_blueprint) 0)
    (set `self.bOutOfAmmo` true)
    (else
      (set `self.bOutOfAmmo` false))))

(event `self.Fire`
  (params (FireDirection :type "Vector Structure"))
  (bind _asgun_blueprint (cast `/Game/Blueprints/GunBlueprint` (`ChildActorComponent.ChildActor` (`self.Gun`))))
  (`/Game/Blueprints/GunBlueprint.Fire` _asgun_blueprint (+ (* (`KismetMathLibrary.RandomUnitVector`) (`self.TargetAccuracyOffset`)) FireDirection))
  (`self.K2_SetActorRotation` (`KismetMathLibrary.Conv_VectorToRotator` FireDirection)))

(event `self.Reload`
  (bind _reloadanimationlength (`self.ReloadStart`))
  (`KismetSystemLibrary.Delay` _reloadanimationlength)
  (`self.ReloadEnd`))

(fn `ReloadEnd`
  (bind _asgun_blueprint (cast `/Game/Blueprints/GunBlueprint` (`ChildActorComponent.ChildActor` (`self.Gun`))))
  (set `self.bIsReloading` false)
  (set `self.bOutOfAmmo` false)
  (`/Game/Blueprints/GunBlueprint.Reload` _asgun_blueprint))

(fn `ReloadStart`
  (returns (ReloadAnimationLength :type "Float (double-precision)"))
  (bind _returnvalue (`AnimInstance.Montage_Play` (`SkeletalMeshComponent.GetAnimInstance` (`self.Mesh`)) "/Game/Assets/Mannequin/AnimStarterPack/ReloadRifleHip_Montage.ReloadRifleHip_Montage" 1.0 "MontageLength" 0.0 true))
  (bind _asgun_blueprint (cast `/Game/Blueprints/GunBlueprint` (`ChildActorComponent.ChildActor` (`self.Gun`))))
  (set `/Game/Blueprints/GunBlueprint.RoundsRemainingInMagazine` 0 _asgun_blueprint)
  (set `/Game/Blueprints/GunBlueprint.bCanFire` false _asgun_blueprint)
  (set `self.bIsReloading` true)
  (return _returnvalue))

(fn `UserConstructionScript`)