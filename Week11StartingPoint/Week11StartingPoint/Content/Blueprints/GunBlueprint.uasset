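; Networked gun attached to the player character, with magazine ammo, fire-rate cooldown and reload.
; Fire traces a predicted projectile arc for an instant hit with debug drawing, plays sound, montage and impact effects, and damages HealthComponents on the server.
; Authority updates cooldown and rounds when firing, while RepNotifies refresh the owning player's ammo HUD.
; CalculateShotDirection provides accuracy-weighted random spread, but Fire does not call it.
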(event `self.ReceiveBeginPlay`
  (set `self.RoundsRemainingInMagazine` (`self.MagazineSize`))
  (`self.UpdateAmmoHUD`))

(event `self.ReceiveTick`
  (params (DeltaSeconds :type "Float (single-precision)"))
  (`/Engine/EditorBlueprintResources/ActorMacros.Switch Has Authority`
    (:`Authority`
      (if (not (`self.bCanFire`))
        (bind _output_get (set `self.TimeTillNextShot` (- (`self.TimeTillNextShot`) DeltaSeconds)))
        (if (<= _output_get 0.0)
          (set `self.bCanFire` (> (`self.RoundsRemainingInMagazine`) 0)))))))

(fn `CalculateShotDirection`
  (params (OriginalDirection :type "Vector Structure"))
  (returns (LaunchDirection :type "Vector Structure"))
  (return (* (`KismetMathLibrary.Normal` (+ (`KismetMathLibrary.RandomUnitVector`) (* OriginalDirection (`self.WeaponAccuracy`)))) (`self.MuzzleVelocity`))))

(fn `Fire`
  (params (LaunchDirection :type "Vector Structure"))
  (bind _returnvalue (`SceneComponent.K2_GetComponentLocation` (`self.MuzzlePosition`)))
  (if (`self.bCanFire`)
    (`/Engine/EditorBlueprintResources/ActorMacros.Switch Has Authority`
      (:`Authority`
        (set `self.bCanFire` false)
        (set `self.TimeTillNextShot` (`self.FireRate`))
        (set `self.RoundsRemainingInMagazine` (- (`self.RoundsRemainingInMagazine`) 1)))
      (:`Remote`
        _))
    (bind _outhit (`GameplayStatics.Blueprint_PredictProjectilePath_ByTraceChannel` :`StartPos` _returnvalue :`LaunchVelocity` (* LaunchDirection (`self.MuzzleVelocity`)) :`ProjectileRadius` 1.0 :`DrawDebugType` "ForDuration" :`DrawDebugTime` 4.0))
    (`GameplayStatics.PlaySoundAtLocation` "/Game/Assets/Audio/FirstPersonTemplateWeaponFire02.FirstPersonTemplateWeaponFire02" _returnvalue (struct) 1.0 1.0 0.0 null null null)
    (bind _asplayer_character_blueprint (cast `/Game/Blueprints/PlayerCharacterBlueprint` (`self.GetParentActor`))
      (:`then`
        (`AnimInstance.Montage_Play` (`SkeletalMeshComponent.GetAnimInstance` (`/Game/Blueprints/PlayerCharacterBlueprint.Arms` _asplayer_character_blueprint)) "/Game/Assets/Arms/Animations/FirstPersonFire_Montage.FirstPersonFire_Montage" 1.0 "MontageLength" 0.0 true))
      (:`CastFailed`
        _))
    (bind (_bblockinghit _binitialoverlap _time _distance _location _impactpoint _normal _impactnormal _physmat _hitactor) (`GameplayStatics.BreakHitResult` _outhit))
    (if (`KismetSystemLibrary.IsValid` _hitactor)
      (bind _returnvalue_2 (`self.GetComponentByClass` _hitactor "/Script/AdvGamesProgramming.HealthComponent"))
      (if (`KismetSystemLibrary.IsValid` _returnvalue_2)
        (`GameplayStatics.SpawnEmitterAtLocation` "/Game/Effects/PlayerHitEffect.PlayerHitEffect" _impactpoint (`KismetMathLibrary.MakeRotFromZ` _impactnormal))
        (if (`KismetSystemLibrary.IsServer`)
          (`HealthComponent.OnTakeDamage` _returnvalue_2 (`self.BulletDamage`))
          (`KismetSystemLibrary.PrintString` (`KismetStringLibrary.Conv_DoubleToString` (`HealthComponent.CurrentHealth` _returnvalue_2)) true false))
        (else
          (`GameplayStatics.SpawnEmitterAtLocation` "/Game/Effects/GroundHitEffect.GroundHitEffect" _impactpoint)
          (`KismetSystemLibrary.PrintString` "Did not hit actor with health component" true false))))))

(fn `OnRep_MagazineSize`
  (`self.UpdateAmmoHUD`))

(fn `OnRep_RoundsRemainingInMagazine`
  (`self.UpdateAmmoHUD`))

(fn `Reload`
  (set `self.RoundsRemainingInMagazine` (`self.MagazineSize`)))

(fn `UpdateAmmoHUD`
  (bind _asplayer_character_blueprint (cast `/Game/Blueprints/PlayerCharacterBlueprint` (`self.GetParentActor`)))
  (if (or (`Pawn.IsLocallyControlled` _asplayer_character_blueprint) (`|EnumEquality` (`self.GetLocalRole` _asplayer_character_blueprint) "ROLE_AutonomousProxy"))
    (bind _asplayer_controller (cast `PlayerController` (`Pawn.GetController` _asplayer_character_blueprint)))
    (bind _asplayer_hud (cast `PlayerHUD` (`PlayerController.GetHUD` _asplayer_controller)))
    (`PlayerHUD.SetAmmoText` _asplayer_hud (`self.RoundsRemainingInMagazine`) (`self.MagazineSize`))))

(fn `UserConstructionScript`)